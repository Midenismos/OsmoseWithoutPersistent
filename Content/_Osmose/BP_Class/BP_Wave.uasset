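; BP_Wave is an expanding wave that follows the Wisp and temporarily swaps the materials of actors it reaches.
; StartExpand shows the mesh, enables sphere collision and plays a timeline that scales the mesh toward ExtensionRange, then reverses and clears the Wisp's WaveLaunched flag.
; Sphere overlaps apply WaveMaterial through message calls, caching each actor's starting material in a map to restore when the overlap ends.
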(event `self.ReceiveTick`
  (params (DeltaSeconds :type "Float (single-precision)"))
  (`self.K2_SetActorLocation` (`self.K2_GetActorLocation` (`self.Wisp`))))

(event `StartExpand`
  (`PrimitiveComponent.SetCollisionEnabled` (`self.Sphere`) "QueryAndPhysics")
  (`SceneComponent.SetHiddenInGame` (`self.StaticMeshComponent`) false false)
  (set `self.HasExpanded` false)
  (bind (_direction _expansionratio) (`Timeline|Extand` :!via `PlayFromStart` :!label _label)
    (:`Update`
      (`SceneComponent.SetWorldScale3D` (`self.StaticMeshComponent`) (`KismetMathLibrary.Conv_DoubleToVector` (* _expansionratio (/ (`self.ExtensionRange`) (`self.SizeAtOneScale`))))))
    (:`Finished`
      (if (`self.HasExpanded`)
        (set `/Game/_Osmose/BP_Class/Wisp.WaveLaunched` false (`self.Wisp`))
        (else
          (set `self.HasExpanded` true)
          (goto _label :!via `ReverseFromEnd`))))))

(event `self.ReceiveBeginPlay`
  (set `self.SizeAtOneScale` (`.SphereRadius` (`KismetSystemLibrary.GetComponentBounds` (`self.StaticMeshComponent`)))))

(event `self.Sphere.OnComponentBeginOverlap`
  (params (OverlappedComponent :type "PrimitiveComponent Object Reference") (OtherActor :type "Actor Object Reference") (OtherComp :type "PrimitiveComponent Object Reference") (OtherBodyIndex :type Integer) (bFromSweep :type Boolean) (SweepResult :type "HitResult Structure (by ref)"))
  (bind _startingmaterials (`self.StartingMaterials`))
  ;[1 1 1] ApplyWaveMaterial
  (bind _startingmaterial (message `/Game/_Osmose/BP_Class/Appropriation_InterfaceEnum/Appropriable.ApplyWaveMaterial` OtherActor (`self.WaveMaterial`)))
  (if (!= _startingmaterial null)
    (`BlueprintMapLibrary.Map_Add` _startingmaterials OtherActor _startingmaterial)
    (else
      (bind _startingmaterial_2 (message `/Game/_Osmose/BP_Class/Possessables/_StructureSystem/Possessable.ApplyWaveMaterial` OtherActor (`self.WaveMaterial`)))
      (`BlueprintMapLibrary.Map_Add` _startingmaterials OtherActor _startingmaterial_2))))

(event `self.Sphere.OnComponentEndOverlap`
  (params (OverlappedComponent :type "PrimitiveComponent Object Reference") (OtherActor :type "Actor Object Reference") (OtherComp :type "PrimitiveComponent Object Reference") (OtherBodyIndex :type Integer))
  (bind _value (`BlueprintMapLibrary.Map_Find` (`self.StartingMaterials`) OtherActor))
  ;[1 1 1] RemoveWaveMaterial
  (message `/Game/_Osmose/BP_Class/Appropriation_InterfaceEnum/Appropriable.ReApplyStartingMaterial` OtherActor _value)
  (message `/Game/_Osmose/BP_Class/Possessables/_StructureSystem/Possessable.ReApplyStartingMaterial` OtherActor _value)
  (`BlueprintMapLibrary.Map_Remove` (`self.StartingMaterials`) OtherActor))

(fn `UserConstructionScript`)